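; TrackGenerator is a construction-script Blueprint that builds a looping track from spline meshes along its Spline component.
; It stores the spline point count, resizes RoadDataArray to match, then calls BuildTrackElement with RoadMesh over the point indices.
; Each element adds a spline mesh using the current and next points' local locations and tangents, with modulo wrapping to close the loop.
; RoadDataArray is only resized here, not read for mesh building.
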(fn `Build Track Element`
  (params (LoopIndex :type Integer) (TrackElementMesh :type "StaticMesh Object Reference"))
  (locals (Local_CurrentLoopIndex :type Integer) (Local_NextLoopIndex :type Integer) (Local_TrackElementMesh :type "StaticMesh Object Reference") (Local_StartLocation :type "Vector Structure") (Local_StartTangent :type "Vector Structure") (Local_EndLocation :type "Vector Structure") (Local_EndTangent :type "Vector Structure") (Local_CurrentSplineMesh :type "SplineMeshComponent Object Reference"))
  (bind (_location _tangent) (`SplineComponent.GetLocationAndTangentAtSplinePoint` (`self.Spline`) (`local.Local_NextLoopIndex`) "Local"))
  (bind (_location_2 _tangent_2) (`SplineComponent.GetLocationAndTangentAtSplinePoint` (`self.Spline`) (`local.Local_CurrentLoopIndex`) "Local"))
  (set `local.Local_CurrentLoopIndex` LoopIndex)
  (set `local.Local_NextLoopIndex` (mod (+ LoopIndex 1) (`self.Number of Spline Points`)))
  (set `local.Local_TrackElementMesh` TrackElementMesh)
  (`|ExecutionSequence`
    (:`then_0`
      (set `local.Local_StartLocation` _location_2)
      (set `local.Local_StartTangent` _tangent_2)
      (set `local.Local_EndLocation` _location)
      (set `local.Local_EndTangent` _tangent))
    (:`then_1`
      (`AddComponent|NODE_AddSplineMeshComponent-0`)
      (`StaticMeshComponent.SetStaticMesh` (`local.Local_CurrentSplineMesh`) (`local.Local_TrackElementMesh`))
      (`SplineMeshComponent.SetStartAndEnd` (`local.Local_CurrentSplineMesh`) (`local.Local_StartLocation`) (`local.Local_StartTangent`) (`local.Local_EndLocation`) (`local.Local_EndTangent`) true))))

(fn `UserConstructionScript`
  (bind _roaddataarray (`self.RoadDataArray`))
  (`|ExecutionSequence`
    (:`then_0`
      (set `self.Number of Spline Points` (`SplineComponent.GetNumberOfSplinePoints` (`self.Spline`))))
    (:`then_1`
      (`/Engine/EditorBlueprintResources/StandardMacros.CompareInt` (`KismetArrayLibrary.Array_Length` (`self.RoadDataArray`)) (`self.Number of Spline Points`) :!label _label
        (:`>`
          (`KismetArrayLibrary.Array_Remove` _roaddataarray (`KismetArrayLibrary.Array_LastIndex` _roaddataarray))
          (goto _label))
        (:`<`
          (`KismetArrayLibrary.Array_Add` (`self.RoadDataArray`))
          (goto _label))))
    (:`then_2`
      (for _index (range (+ (`self.Number of Spline Points`) 1))
        (`self.Build Track Element` _index (`self.RoadMesh`))))
    (:`then_3`)))